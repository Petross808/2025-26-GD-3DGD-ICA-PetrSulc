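; BP_Door is an escape room door that opens when the player selects it while holding a key.
; It implements the Selectable OnSelected event and checks that the held item casts to BP_Key, doing nothing otherwise.
; Opening swaps visibility and collision from the Door component to a separate OpenDoor component rather than animating, then plays player dialogue and a door sound.
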(event OnSelected(Selectable)
  (params (Player :type BP%20First%20Person%20Character%20Object%20Reference))
  (bind _door (Variables|Default|GetDoor))
  (bind _opendoor (Variables|Default|GetOpenDoor))
  (Utilities|Casting|CastToBP_Key (Variables|/Game/FirstPerson/Blueprints/BP_FirstPersonCharacter.BP_FirstPersonCharacter_C|GetHeldItem Player))
  (Rendering|SetVisibility _door false false)
  (Collision|SetCollisionEnabled _door "NoCollision")
  (Rendering|SetVisibility _opendoor true false)
  (Collision|SetCollisionEnabled _opendoor "QueryAndPhysics")
  (Default|PlayDialogue Player "Finally got the door open..." 3.0)
  (Audio|PlaySoundatLocation "/Game/EscapeRoom/SoundEffects/SW_Door.SW_Door" (Transformation|GetActorLocation) "0, 0, 0" 1.0 1.0 0.3 0 0 0 0))

(event EventBeginPlay)

(event Collision|EventActorBeginOverlap
  (params (OtherActor :type Actor%20Object%20Reference)))

(event EventTick
  (params (DeltaSeconds :type Float%20%28single-precision%29)))

(fn ConstructionScript)
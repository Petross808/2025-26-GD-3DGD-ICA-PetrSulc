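; BP_Globe is an escape room puzzle prop: a globe with a hidden compartment that opens once every referenced book slot holds a book.
; While closed, Tick polls the BookSlots array and fires OpenGlobe once when all slots have valid books.
; OpenGlobe swaps the closed top mesh for the open one, disables the Box collision and plays a sound.
; Selecting the globe has the player examine it, showing a latch hint with a sound.
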(event OnSelected(Selectable)
  (params (Player :type BP%20First%20Person%20Character%20Object%20Reference))
  (Default|ExamineActor Player self "Globe" "There is a suspicious latch on the back. I wonder if there's a secret compartment." 4.0)
  (Audio|PlaySoundatLocation "/Game/EscapeRoom/SoundEffects/SW_Examine.SW_Examine" (Transformation|GetActorLocation) "0, 0, 0" 1.0 1.0 0.0 0 0 0 0))

(event Custom|OpenGlobe
  (Rendering|SetVisibility (Variables|Default|GetGlobeTopClosed) false false)
  (Rendering|SetVisibility (Variables|Default|GetGlobeTop) true false)
  (Collision|SetCollisionEnabled (Variables|Default|GetBox) "NoCollision")
  (Audio|PlaySoundatLocation "/Game/EscapeRoom/SoundEffects/SW_OpenGlobe.SW_OpenGlobe" (Transformation|GetActorLocation) "0, 0, 0" 1.0 1.0 0.0 0 0 0 0))

(event EventBeginPlay)

(event Collision|EventActorBeginOverlap
  (params (OtherActor :type Actor%20Object%20Reference)))

(event EventTick
  (params (DeltaSeconds :type Float%20%28single-precision%29))
  (if (Variables|Default|GetClosed)
    (Variables|Default|SetShouldOpen true)
    (for _array_element (Variables|Default|GetBookSlots)
      (Variables|/Game/EscapeRoom/ActorBPs/BP_BookSlot.BP_BookSlot_C|GetBook _array_element
        (:then)
        (:else
          (Variables|Default|SetShouldOpen false))))
    (if (Variables|Default|GetShouldOpen)
      (Variables|Default|SetClosed false)
      (CallFunction|OpenGlobe))))

(fn ConstructionScript)